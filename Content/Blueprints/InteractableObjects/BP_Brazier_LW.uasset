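; Interactable brazier that toggles its small fire particle effect and fades its point light on each interaction.
; Interact drives two FlipFlops: one switches the particles and swaps the widget between alternative and initial text, rebuilding it.
; The other plays or reverses a timeline that lerps light intensity between LightIntensity and zero.
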(event Collision|EventActorBeginOverlap
  (params (OtherActor :type Actor%20Object%20Reference))
  (|CallParentFunction OtherActor) ; This node is disabled and will not be called.\nDrag off pins to build functionality.
)

(event EventTick
  (params (DeltaSeconds :type Float%20%28single-precision%29))
  (|CallParentFunction DeltaSeconds) ; This node is disabled and will not be called.\nDrag off pins to build functionality.
)

(event EventInteract
  (bind _ps_fx_fire_small (Variables|Default|GetPS_FX_Fire_Small))
  ;[1 1 1] Toggle fire
  (Utilities|FlowControl|FlipFlop
    (:A
      (Variables|Default|SetWidgetText (Variables|Default|GetAlternativeWidgetText))
      (CallFunction|RebuildWidget)
      (Components|Activation|SetActive _ps_fx_fire_small true false))
    (:B
      (Variables|Default|SetWidgetText (Variables|Default|GetInitialWidgetText))
      (CallFunction|RebuildWidget)
      (Components|Activation|SetActive _ps_fx_fire_small false false)))
  ;[1 1 1] Fade in/out light
  (Utilities|FlowControl|FlipFlop
    (:A
      (bind _newtrack_0 (Timeline|Timeline Play)
        (:Update
          (Rendering|Components|Light|SetIntensity (Variables|Default|GetPointLight) (Math|Float|Lerp (Variables|Default|GetLightIntensity) 0.0 _newtrack_0)))))
    (:B
      (Timeline|Timeline Reverse))))

(fn ConstructionScript
  (|CallParentFunction))