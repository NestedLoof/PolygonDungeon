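; Interactable chest that highlights and shows an interaction prompt when the player character enters its trigger box; no opening logic is defined here.
; Overlap toggles custom depth on both meshes, the widget's visibility and player input, clearing them on exit or when not interactable.
; The prompt is created on BeginPlay with configurable text, and helper functions rebuild it or expose its component.
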(event OnComponentBeginOverlap(Box)
  (params (OverlappedComponent :type Primitive%20Component%20Object%20Reference) (OtherActor :type Actor%20Object%20Reference) (OtherComp :type Primitive%20Component%20Object%20Reference) (OtherBodyIndex :type Integer) (bFromSweep :type Boolean) (SweepResult :type Hit%20Result%20Structure%20%28by%20ref%29))
  (bind _returnvalue (Game|GetPlayerController 0))
  (bind _object (Variables|Default|GetObject))
  (bind _parentmesh (Variables|Default|GetParentMesh))
  (bind _interactwidget (Variables|Default|GetInteractWidget))
  ;[1 1 1] Highlight the interactable object
  (if (Variables|Default|GetInteractable)
    (Utilities|Casting|CastToBP_Character_LW OtherActor)
    (Input|EnableInput _returnvalue)
    (Rendering|SetRenderCustomDepth _object true)
    (Rendering|SetRenderCustomDepth _parentmesh true)
    (Utilities|IsValid _interactwidget
      (:Is%20Valid
        (Development|SetHiddeninGame _interactwidget false false)))
    (else
      ;[1 1 1] Un-highlight the object
      (Utilities|Casting|CastToBP_Character_LW (stale OnComponentEndOverlap(Box) OtherActor))
      (Input|DisableInput _returnvalue 0)
      (Rendering|SetRenderCustomDepth _object false)
      (Rendering|SetRenderCustomDepth _parentmesh false)
      (Utilities|IsValid _interactwidget
        (:Is%20Valid
          (Development|SetHiddeninGame _interactwidget true false))))))

(event OnComponentEndOverlap(Box)
  (params (OverlappedComponent :type Primitive%20Component%20Object%20Reference) (OtherActor :type Actor%20Object%20Reference) (OtherComp :type Primitive%20Component%20Object%20Reference) (OtherBodyIndex :type Integer))
  (bind _interactwidget (Variables|Default|GetInteractWidget))
  ;[1 1 1] Un-highlight the object
  (Utilities|Casting|CastToBP_Character_LW OtherActor)
  (Input|DisableInput (Game|GetPlayerController 0) 0)
  (Rendering|SetRenderCustomDepth (Variables|Default|GetObject) false)
  (Rendering|SetRenderCustomDepth (Variables|Default|GetParentMesh) false)
  (Utilities|IsValid _interactwidget
    (:Is%20Valid
      (Development|SetHiddeninGame _interactwidget true false))))

(event EventBeginPlay
  (CallFunction|InitialiseWidget))

(fn ConstructionScript)

(fn InitialiseWidget
  (bind _returnvalue (UserInterface|CreateWidget "/Game/Blueprints/UI/WBP_Interaction_LW.WBP_Interaction_LW_C"))
  (UserInterface|SetWidget (Variables|Default|GetInteractWidget) _returnvalue)
  (bind _output_get (Variables|Default|SetDisplayWidget _returnvalue))
  (Variables|/Game/Blueprints/UI/WBP_Interaction_LW.WBP_Interaction_LW_C|SetItemName _output_get (Variables|Default|GetInitialWidgetText)))

(fn RebuildWidget
  (Widget|RemovefromParent (Variables|Default|GetDisplayWidget))
  (Utilities|Platform|CollectGarbage)
  (CallFunction|InitialiseWidget))

(fn GetInteractionWidgetRef
  (return (Variables|Default|GetInteractWidget)))