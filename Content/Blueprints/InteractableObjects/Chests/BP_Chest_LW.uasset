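; BP_Chest_LW is an interactable chest with a two-stage interaction: open it, then take the item inside.
; The first interact plays a Timeline that rotates the lid from its cached rotation and brightens a point light.
; When finished, the prompt takes the item's name from its DataTable row, with fallback text.
; The next interact adds the item to the player's inventory, refreshes the inventory menu and disables the chest.
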(event EventBeginPlay
  (|CallParentFunction) ; This node is disabled and will not be called.\nDrag off pins to build functionality.
)

(event Collision|EventActorBeginOverlap
  (params (OtherActor :type Actor%20Object%20Reference))
  (|CallParentFunction OtherActor) ; This node is disabled and will not be called.\nDrag off pins to build functionality.
)

(event EventTick
  (params (DeltaSeconds :type Float%20%28single-precision%29))
  (|CallParentFunction DeltaSeconds) ; This node is disabled and will not be called.\nDrag off pins to build functionality.
)

(event EventInteract
  (bind _returnvalue (Game|GetPlayerCharacter 0))
  (bind _asbp_character_lw (Utilities|Casting|CastToBP_Character_LW _returnvalue))
  (if (Variables|Default|GetInteractable)
    (if (Variables|Default|GetChestOpened)
      ;[1 1 1] take item
      (Variables|Default|SetInteractable false)
      (Rendering|Components|Light|SetIntensity (Variables|Default|GetPointLight) 0.0)
      (Default|AddItemtoInventory (Variables|Default|GetItemDataComponent) _asbp_character_lw)
      (Components|DestroyComponent (Variables|Default|GetInteractWidget))
      (Default|DisplayInventory (Variables|/Game/Blueprints/HUD/WBP_HUD_LW.WBP_HUD_LW_C|GetInventoryMenu (Variables|/Game/Blueprints/Characters/BP_Character_LW.BP_Character_LW_C|GetHudRef _asbp_character_lw)))
      (else
        ;[1 1 1] open chest
        (bind _newtrack_0 (Timeline|Timeline Play)
          (:Update
            (CallFunction|OpenDoor _newtrack_0)
            (CallFunction|IncreaseLight _newtrack_0))
          (:Finished
            (CallFunction|UpdateWidgetTextforItem)
            (Variables|Default|SetChestOpened true)))))))

(fn ConstructionScript
  (|CallParentFunction)
  (Variables|Default|SetInitialRotation (Variables|/Script/Engine.SceneComponent|GetRelativeRotation (Variables|Default|GetObject))))

(fn OpenDoor
  (params (Roll :type Float%20%28single-precision%29))
  (Transformation|SetRelativeRotation (Variables|Default|GetObject) (Math|Rotator|CombineRotators (Math|Rotator|MakeRotator (* Roll -9e+01) 0.0 0.0) (Variables|Default|GetInitialRotation)) false false))

(fn IncreaseLight
  (params (Alpha :type Float%20%28double-precision%29))
  (Rendering|Components|Light|SetIntensity (Variables|Default|GetPointLight) (Math|Float|Lerp 0.0 (Variables|Default|GetMaxLightIntensity) Alpha)))

(fn UpdateWidgetTextforItem
  (bind _itemdatacomponent (Variables|Default|GetItemDataComponent))
  (bind _itemid (Variables|/Game/Blueprints/Inventory/ItemDataComponent.ItemDataComponent_C|GetItemId _itemdatacomponent))
  (bind _returnvalue (Utilities|GetDataTableRow (.datatable _itemid) (.rowname _itemid))
    (:then
      (Variables|Default|SetInitialWidgetText (Utilities|String|ToString(Text) (Utilities|Text|FormatText "take {item}" (.Name (Utilities|Struct|BreakFInventoryItem _returnvalue))))))
    (:RowNotFound
      (Variables|Default|SetInitialWidgetText (Variables|Default|GetAlternativeWidgetText))))
  (CallFunction|RebuildWidget))