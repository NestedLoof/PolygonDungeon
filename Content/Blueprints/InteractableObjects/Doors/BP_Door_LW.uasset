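; BP_Door_LW is an interactable door that swings open and closed on alternate Interact events.
; A FlipFlop plays or reverses a Timeline, whose track adds yaw to the Object component's initial relative rotation, captured in the construction script.
; Each toggle also switches the widget text between its initial and alternative strings and rebuilds the widget.
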(event EventBeginPlay
  (|CallParentFunction) ; This node is disabled and will not be called.\nDrag off pins to build functionality.
)

(event Collision|EventActorBeginOverlap
  (params (OtherActor :type Actor%20Object%20Reference))
  (|CallParentFunction OtherActor) ; This node is disabled and will not be called.\nDrag off pins to build functionality.
)

(event EventTick
  (params (DeltaSeconds :type Float%20%28single-precision%29))
  (|CallParentFunction DeltaSeconds) ; This node is disabled and will not be called.\nDrag off pins to build functionality.
)

(event EventInteract
  ;[1 1 1] Open/close the door
  (Utilities|FlowControl|FlipFlop
    (:A
      (Variables|Default|SetWidgetText (Variables|Default|GetAlternativeWidgetText))
      (CallFunction|RebuildWidget)
      (bind _newtrack_0 (Timeline|Timeline Play)
        (:Update
          (Transformation|SetRelativeRotation (Variables|Default|GetObject) (Math|Rotator|CombineRotators (Math|Rotator|MakeRotator 0.0 0.0 _newtrack_0) (Variables|Default|GetInitialRotation)) false false))))
    (:B
      (Variables|Default|SetWidgetText (Variables|Default|GetInitialWidgetText))
      (CallFunction|RebuildWidget)
      (Timeline|Timeline Reverse))))

(fn ConstructionScript
  (|CallParentFunction)
  (Variables|Default|SetInitialRotation (Variables|/Script/Engine.SceneComponent|GetRelativeRotation (Variables|Default|GetObject))))