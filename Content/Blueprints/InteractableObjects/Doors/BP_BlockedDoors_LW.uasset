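; Interactable double door that the player can open only from its openable side, with a different prompt on the blocked side.
; Two collision boxes set the widget text, enable input and toggle custom depth highlighting, rebuilding the widget with forced garbage collection on each text change.
; Interact plays a timeline that swings the doors in opposite yaw from Door2's initial rotation, then disables further interaction.
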(event OnComponentBeginOverlap(CollisionBoxBlocked)
  (params (OverlappedComponent :type Primitive%20Component%20Object%20Reference) (OtherActor :type Actor%20Object%20Reference) (OtherComp :type Primitive%20Component%20Object%20Reference) (OtherBodyIndex :type Integer) (bFromSweep :type Boolean) (SweepResult :type Hit%20Result%20Structure%20%28by%20ref%29))
  (bind _returnvalue (Game|GetPlayerController 0))
  (bind _door1mesh (Variables|Default|GetDoor1Mesh))
  (bind _interactwidget (Variables|Default|GetInteractWidget))
  ;[1 1 1] Highlight the interactable object
  (Utilities|Casting|CastToBP_Character_LW OtherActor)
  (if (Variables|Default|GetInteractable)
    (Variables|Default|SetWidgetText (Variables|Default|GetInitialWidgetText))
    (CallFunction|RebuildWidget)
    (Input|EnableInput _returnvalue)
    (Rendering|SetRenderCustomDepth _door1mesh true)
    (Development|SetHiddeninGame _interactwidget false false)
    (else
      ;[1 1 1] Un-highlight the object
      (Utilities|Casting|CastToBP_Character_LW (stale OnComponentEndOverlap(CollisionBoxBlocked) OtherActor))
      (Input|DisableInput _returnvalue 0)
      (Rendering|SetRenderCustomDepth _door1mesh false)
      (Development|SetHiddeninGame _interactwidget true false))))

(event OnComponentEndOverlap(CollisionBoxBlocked)
  (params (OverlappedComponent :type Primitive%20Component%20Object%20Reference) (OtherActor :type Actor%20Object%20Reference) (OtherComp :type Primitive%20Component%20Object%20Reference) (OtherBodyIndex :type Integer))
  ;[1 1 1] Un-highlight the object
  (Utilities|Casting|CastToBP_Character_LW OtherActor)
  (Input|DisableInput (Game|GetPlayerController 0) 0)
  (Rendering|SetRenderCustomDepth (Variables|Default|GetDoor1Mesh) false)
  (Development|SetHiddeninGame (Variables|Default|GetInteractWidget) true false))

(event OnComponentBeginOverlap(CollisionBoxOpenable)
  (params (OverlappedComponent :type Primitive%20Component%20Object%20Reference) (OtherActor :type Actor%20Object%20Reference) (OtherComp :type Primitive%20Component%20Object%20Reference) (OtherBodyIndex :type Integer) (bFromSweep :type Boolean) (SweepResult :type Hit%20Result%20Structure%20%28by%20ref%29))
  (bind _returnvalue (Game|GetPlayerController 0))
  (bind _door1mesh (Variables|Default|GetDoor1Mesh))
  (bind _interactwidget (Variables|Default|GetInteractWidget))
  ;[1 1 1] Highlight the interactable object
  (Utilities|Casting|CastToBP_Character_LW OtherActor)
  (if (Variables|Default|GetInteractable)
    (Variables|Default|SetWidgetText (Variables|Default|GetAlternativeWidgetText))
    (CallFunction|RebuildWidget)
    (Input|EnableInput _returnvalue)
    (Rendering|SetRenderCustomDepth _door1mesh true)
    (Development|SetHiddeninGame _interactwidget false false)
    (else
      ;[1 1 1] Un-highlight the object
      (Utilities|Casting|CastToBP_Character_LW (stale OnComponentEndOverlap(CollisionBoxBlocked) OtherActor))
      (Input|DisableInput _returnvalue 0)
      (Rendering|SetRenderCustomDepth _door1mesh false)
      (Development|SetHiddeninGame _interactwidget true false))))

(event OnComponentEndOverlap(CollisionBoxOpenable)
  (params (OverlappedComponent :type Primitive%20Component%20Object%20Reference) (OtherActor :type Actor%20Object%20Reference) (OtherComp :type Primitive%20Component%20Object%20Reference) (OtherBodyIndex :type Integer))
  ;[1 1 1] Un-highlight the object
  (Utilities|Casting|CastToBP_Character_LW OtherActor)
  (Input|DisableInput (Game|GetPlayerController 0) 0)
  (Rendering|SetRenderCustomDepth (Variables|Default|GetDoor1Mesh) false)
  (Development|SetHiddeninGame (Variables|Default|GetInteractWidget) true false))

(event EventBeginPlay
  (CallFunction|InitialiseWidget))

(event EventInteract
  ;[1 1 1] Open doors
  (if (Variables|Default|GetInteractable)
    (if (Collision|IsOverlappingActor (Variables|Default|GetCollisionBoxOpenable) (Game|GetPlayerCharacter 0) :!class /Script/Engine.PrimitiveComponent)
      (bind _newtrack_0 (Timeline|Timeline Play)
        (:Update
          (Transformation|SetRelativeRotation (Variables|Default|GetDoor2Mesh) (Math|Rotator|CombineRotators (Math|Rotator|MakeRotator 0.0 0.0 _newtrack_0) (Variables|Default|GetInitialRotation)) false false)
          (Transformation|SetRelativeRotation (Variables|Default|GetDoor1Mesh) (Math|Rotator|CombineRotators (Math|Rotator|MakeRotator 0.0 0.0 (* _newtrack_0 -1.0)) (Variables|Default|GetInitialRotation)) false false)
          (Variables|Default|SetInteractable false))))))

(fn ConstructionScript
  (Variables|Default|SetInitialRotation (Variables|/Script/Engine.SceneComponent|GetRelativeRotation (Variables|Default|GetDoor2Mesh))))

(fn InitialiseWidget
  (bind _returnvalue (UserInterface|CreateWidget "/Game/Blueprints/UI/WBP_Interaction_LW.WBP_Interaction_LW_C"))
  (UserInterface|SetWidget (Variables|Default|GetInteractWidget) _returnvalue)
  (bind _output_get (Variables|Default|SetDisplayWidget _returnvalue))
  (Variables|/Game/Blueprints/UI/WBP_Interaction_LW.WBP_Interaction_LW_C|SetItemName _output_get (Variables|Default|GetWidgetText)))

(fn RebuildWidget
  (Widget|RemovefromParent (Variables|Default|GetDisplayWidget))
  (Utilities|Platform|CollectGarbage)
  (CallFunction|InitialiseWidget))

(fn GetInteractionWidgetRef
  (return 0))