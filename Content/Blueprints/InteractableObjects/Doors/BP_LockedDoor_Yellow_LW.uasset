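; Interactable locked door that needs a key item from the player's inventory before it swings open and closed.
; Interact checks for the key, then UnlockDoor shows a VFX, drops the lock mesh with physics, consumes the key and refreshes the inventory display.
; After a short delay, or immediately if already unlocked, a FlipFlop swaps the prompt text and plays or reverses a yaw Timeline relative to the initial rotation.
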(event EventBeginPlay
  (|CallParentFunction) ; This node is disabled and will not be called.\nDrag off pins to build functionality.
)

(event Collision|EventActorBeginOverlap
  (params (OtherActor :type Actor%20Object%20Reference))
  (|CallParentFunction OtherActor) ; This node is disabled and will not be called.\nDrag off pins to build functionality.
)

(event EventTick
  (params (DeltaSeconds :type Float%20%28single-precision%29))
  (|CallParentFunction DeltaSeconds) ; This node is disabled and will not be called.\nDrag off pins to build functionality.
)

(event EventInteract
  (if (Variables|Default|GetLocked)
    ;[1 1 1] Try to unlock the door
    (if (CallFunction|PlayerHasKey (Variables|Default|GetKey%20Item%20Id))
      (CallFunction|UnlockDoor)
      (Utilities|FlowControl|Delay 0.5)
      ;[1 1 1] Open/close the door
      (Utilities|FlowControl|FlipFlop :!label _label
        (:A
          (Variables|Default|SetWidgetText (Variables|Default|GetAlternativeWidgetText))
          (CallFunction|RebuildWidget)
          (bind _newtrack_0 (Timeline|Timeline Play)
            (:Update
              (Transformation|SetRelativeRotation (Variables|Default|GetObject) (Math|Rotator|CombineRotators (Math|Rotator|MakeRotator 0.0 0.0 _newtrack_0) (Variables|Default|GetInitialRotation)) false false))))
        (:B
          (Variables|Default|SetWidgetText (Variables|Default|GetInitialWidgetText))
          (CallFunction|RebuildWidget)
          (Timeline|Timeline Reverse))))
    (else
      (goto _label))))

(fn ConstructionScript
  (|CallParentFunction)
  (Variables|Default|SetInitialRotation (Variables|/Script/Engine.SceneComponent|GetRelativeRotation (Variables|Default|GetObject))))

(fn PlayerHasKey
  (params (ItemId :type Name))
  (bind _foundslot (Default|FindSlot (Variables|/Game/Blueprints/Characters/BP_Character_LW.BP_Character_LW_C|GetInventory (.AsBP%20Character%20LW (Utilities|Casting|CastToBP_Character_LW (Game|GetPlayerCharacter 0)))) ItemId))
  (if _foundslot
    (return true)))

(fn UnlockDoor
  ;[1 1 1] Unlock door
  (Development|SetHiddeninGame (Variables|Default|GetLocked_VFX) false false)
  (Physics|SetSimulatePhysics (Variables|Default|GetLockMesh) true)
  (Variables|Default|SetInitialWidgetText "open door")
  (Variables|Default|SetLocked false)
  ;[1 1 1] Remove key from inventory
  (bind _asbp_character_lw (Utilities|Casting|CastToBP_Character_LW (Game|GetPlayerCharacter 0)))
  (Default|RemovefromInventory (Variables|/Game/Blueprints/Characters/BP_Character_LW.BP_Character_LW_C|GetInventory _asbp_character_lw) (Variables|Default|GetKey%20Item%20Id) 1)
  (Default|DisplayInventory (Variables|/Game/Blueprints/HUD/WBP_HUD_LW.WBP_HUD_LW_C|GetInventoryMenu (Variables|/Game/Blueprints/Characters/BP_Character_LW.BP_Character_LW_C|GetHudRef _asbp_character_lw)))
  (return))