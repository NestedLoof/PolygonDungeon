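; Interactable great sword pickup that the player takes to wield as a weapon.
; The construction script applies the WeaponMesh variable to its static mesh component.
; On Interact, it casts the player character to BP_Character_LW, passes that mesh to WieldWeapon, then destroys itself.
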(event EventBeginPlay
  (|CallParentFunction) ; This node is disabled and will not be called.\nDrag off pins to build functionality.
)

(event Collision|EventActorBeginOverlap
  (params (OtherActor :type Actor%20Object%20Reference))
  (|CallParentFunction OtherActor) ; This node is disabled and will not be called.\nDrag off pins to build functionality.
)

(event EventTick
  (params (DeltaSeconds :type Float%20%28single-precision%29))
  (|CallParentFunction DeltaSeconds) ; This node is disabled and will not be called.\nDrag off pins to build functionality.
)

(event EventInteract
  ;[1 1 1] Pick up weapon
  (bind _asbp_character_lw (Utilities|Casting|CastToBP_Character_LW (Game|GetPlayerCharacter 0)))
  (Default|WieldWeapon _asbp_character_lw (Variables|Default|GetWeaponMesh))
  (Actor|DestroyActor))

(fn ConstructionScript
  (|CallParentFunction)
  (Components|StaticMesh|SetStaticMesh (Variables|Default|GetObject) (Variables|Default|GetWeaponMesh)))