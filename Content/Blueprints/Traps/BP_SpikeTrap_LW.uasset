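; BP_SpikeTrap_LW is a trap whose spikes cycle up and down and which damages Characters that overlap it.
; From BeginPlay, a short random delay feeds a FlipFlop alternating two Timelines, one forward and one reversed, that set the Spikes' relative Z.
; Each Timeline's Finished loops back to the delay, so movement repeats indefinitely.
; Actor overlap applies the Damage variable independently of spike position, with no explicit state check.
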(event Collision|EventActorBeginOverlap
  (params (OtherActor :type Actor%20Object%20Reference))
  ;[1 1 1] Damage character
  (bind _ascharacter (Utilities|Casting|CastToCharacter OtherActor))
  (Game|Damage|ApplyDamage _ascharacter (Variables|Default|GetDamage) 0 self))

(event EventTick
  (params (DeltaSeconds :type Float%20%28single-precision%29)))

(event EventBeginPlay
  ;[1 1 1] Move spikes
  (Utilities|FlowControl|Delay (Math|Random|RandomFloatinRange 0.25 0.75) :!label _label)
  (Utilities|FlowControl|FlipFlop
    (:A
      (bind _newtrack_0 (Timeline|Timeline_0 PlayFromStart)
        (:Update
          (Transformation|SetRelativeTransform (Variables|Default|GetSpikes) (Math|Transform|MakeTransform (Math|Vector|MakeVector 0.0 0.0 _newtrack_0) "0, 0, 0" "1.000000,1.000000,1.000000") false false))
        (:Finished
          (goto _label))))
    (:B
      (bind _newtrack_0_2 (Timeline|Timeline_2 ReverseFromEnd)
        (:Update
          (Transformation|SetRelativeTransform (Variables|Default|GetSpikes) (Math|Transform|MakeTransform (Math|Vector|MakeVector 0.0 0.0 _newtrack_0_2) "0, 0, 0" "1.000000,1.000000,1.000000") false false))
        (:Finished
          (goto _label))))))

(fn ConstructionScript)