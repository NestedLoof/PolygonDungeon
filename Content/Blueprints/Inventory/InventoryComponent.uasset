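; Inventory component that stores items as stacks in a fixed-size slot array, seeded at BeginPlay with one test coin.
; Adding works unit by unit, topping up stacks below the DT_Item stack size, then claiming zero-quantity slots, and reports any remainder.
; Removal shares FindSlot, so it skips full stacks and can match depleted slots, which keep their ItemId.
; Key 1 prints the contents for debugging.
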(event EventBeginPlay
  ;[1 1 1] Initialise inventory
  (Utilities|Array|Resize (Variables|Default|GetContent) (Variables|Default|GetInventorySize))
  (CallFunction|AddtoInventory "coin" 1))

(event Input|KeyboardEvents|1
  (params (Key :type Key%20Structure :default "None"))
  ;[1 1 1] DEBUG - press 1 to view inventory
  (:Pressed
    (CallFunction|DEBUGPrintContents)))

(fn AddtoInventory
  (params (ItemId :type Name) (Quantity :type Integer))
  ;[1 1 1] Loop through entire quantity until nothing left, or we failed to add it to inventory
  (LocalVariables|SetLocal_QuantityRemaining Quantity)
  (while (and (> (LocalVariables|GetLocal_QuantityRemaining) 0) (not (LocalVariables|GetLocal_HasFailed)))
    ;[1 1 1] Try to find slot with same item
    (bind (_index _foundslot) (CallFunction|FindSlot ItemId))
    (if _foundslot
      ;[1 1 1] If we find a stack for that item, add it
      (CallFunction|AddtoStack _index 1)
      (Math|Integer|DecrementInt (LocalVariables|GetLocal_QuantityRemaining))
      (else
        ;[1 1 1] If there is no existing stack for that item, create one
        (if (.HasEmptySlot (CallFunction|AnyEmptySlotsAvailable))
          (bind _success (CallFunction|CreateNewStack ItemId 1))
          (if _success
            (Math|Integer|DecrementInt (LocalVariables|GetLocal_QuantityRemaining))
            (else
              (LocalVariables|SetLocal_HasFailed true)))
          (else
            (LocalVariables|SetLocal_HasFailed true))))))
  ;[1 1 1] Return whether we succeeded
  (return (not (LocalVariables|GetLocal_HasFailed)) (LocalVariables|GetLocal_QuantityRemaining)))

(fn RemovefromInventory
  (params (ItemId :type Name) (Quantity :type Integer))
  ;[1 1 1] Loop through entire quantity until nothing left, or we failed to remove it from inventory
  (Variables|Default|SetLocalQuantityRemaining Quantity)
  (while (and (> (Variables|Default|GetLocalQuantityRemaining) 0) (not (Variables|Default|GetLocalHasFailed)))
    ;[1 1 1] Try to find slot with same item
    (bind (_index _foundslot) (CallFunction|FindSlot ItemId))
    (if _foundslot
      ;[1 1 1] If we find a stack for that item, add it
      (CallFunction|RemovefromStack _index 1)
      (Math|Integer|DecrementInt (Variables|Default|GetLocalQuantityRemaining))
      (else
        (Variables|Default|SetLocalHasFailed true))))
  ;[1 1 1] Return whether we succeeded
  (return (not (Variables|Default|GetLocalHasFailed)) (Variables|Default|GetLocalQuantityRemaining)))

(fn FindSlot
  (params (ItemId :type Name))
  (for (_array_element _array_index) (Variables|Default|GetContent)
    (if (== (.ItemId (Utilities|Struct|BreakFInventorySlot _array_element)) ItemId)
      (if (< (.Quantity (Utilities|Struct|BreakFInventorySlot _array_element)) (CallFunction|GetMaxStackSize ItemId))
        (return _array_index true))))
  (return -1 false))

(fn GetMaxStackSize
  (params (ItemId :type Name))
  (bind _returnvalue (Utilities|GetDataTableRow "/Game/Blueprints/Inventory/DT_Item.DT_Item" ItemId)
    (:then
      (return (Utilities|Struct|BreakFInventoryItem _returnvalue)))
    (:RowNotFound
      (return -1))))

(fn AddtoStack
  (params (Index :type Integer) (Quantity :type Integer))
  (bind _content (Variables|Default|GetContent))
  (bind _output (Utilities|Array|Get(acopy) _content Index))
  (Utilities|Array|SetArrayElem (Variables|Default|GetContent) Index (Utilities|Struct|MakeFInventorySlot (.itemid _output) (+ (.quantity _output) Quantity))))

(fn AnyEmptySlotsAvailable
  (for (_array_element _array_index) (Variables|Default|GetContent)
    (if (== (.Quantity (Utilities|Struct|BreakFInventorySlot _array_element)) 0)
      (return true _array_index)))
  (return false -1))

(fn CreateNewStack
  (params (ItemId :type Name) (Quantity :type Integer))
  (bind (_hasemptyslot _emptyindex) (CallFunction|AnyEmptySlotsAvailable))
  (if _hasemptyslot
    (Utilities|Array|SetArrayElem (Variables|Default|GetContent) _emptyindex (Utilities|Struct|MakeFInventorySlot ItemId Quantity))
    (return true)
    (else
      (return false))))

(fn DEBUGPrintContents
  (for (_array_element _array_index) (Variables|Default|GetContent)
    (Development|PrintString (Utilities|String|Append (Utilities|String|ToString(Integer) _array_index) ": " (Utilities|String|ToString(Name) (.ItemId (Utilities|Struct|BreakFInventorySlot _array_element))) " =  " (Utilities|String|ToString(Integer) (.Quantity (Utilities|Struct|BreakFInventorySlot _array_element)))) true true "(R=0.000000,G=0.660000,B=1.000000,A=1.000000)" 5.0)))

(fn RemovefromStack
  (params (Index :type Integer) (Quantity :type Integer))
  (bind _content (Variables|Default|GetContent))
  (bind _output (Utilities|Array|Get(acopy) _content Index))
  (Utilities|Array|SetArrayElem (Variables|Default|GetContent) Index (Utilities|Struct|MakeFInventorySlot (.itemid _output) (- (.quantity _output) Quantity))))