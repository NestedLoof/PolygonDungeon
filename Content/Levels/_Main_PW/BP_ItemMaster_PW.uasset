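; BP_ItemMaster_PW is a pickup item actor, named as a master item, that the player collects by pressing K while nearby.
; Sphere overlap with a BP_Character_LW enables input for the first player controller, and end overlap calls DisableInput.
; On K, it casts the overlapping actor to that character, passes ItemInfoPW to its PickUpItemEvent, then destroys itself.
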(event OnComponentBeginOverlap(Sphere)
  (params (OverlappedComponent :type Primitive%20Component%20Object%20Reference) (OtherActor :type Actor%20Object%20Reference) (OtherComp :type Primitive%20Component%20Object%20Reference) (OtherBodyIndex :type Integer) (bFromSweep :type Boolean) (SweepResult :type Hit%20Result%20Structure%20%28by%20ref%29))
  (Utilities|Casting|CastToBP_Character_LW OtherActor)
  (Input|EnableInput (Game|GetPlayerController 0)))

(event OnComponentEndOverlap(Sphere)
  (params (OverlappedComponent :type Primitive%20Component%20Object%20Reference) (OtherActor :type Actor%20Object%20Reference) (OtherComp :type Primitive%20Component%20Object%20Reference) (OtherBodyIndex :type Integer))
  (Utilities|Casting|CastToBP_Character_LW OtherActor)
  (Input|DisableInput (Game|GetPlayerController 0) 0))

(event Input|KeyboardEvents|K
  (params (Key :type Key%20Structure :default "None"))
  (:Pressed
    (bind _asbp_character_lw (Utilities|Casting|CastToBP_Character_LW (stale OnComponentBeginOverlap(Sphere) OtherActor)))
    (Default|PickUpItemEvent _asbp_character_lw (Variables|Default|GetItemInfo_PW))
    (Actor|DestroyActor)))

(fn ConstructionScript)